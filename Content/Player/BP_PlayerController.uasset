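; Player controller for a voxel-world game that feeds a debug readout of player position and movement mode.
; BeginPlay adds the default Enhanced Input mapping, creates WBP_Interface, and caches references to the VoxelWorld actor and main character.
; Each Tick writes the player's cell coordinate, sector coordinate and Ground/Air movement state into the widget's text lines.
; The widget's AddToViewport call is disconnected, so this controller never displays it.
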(event EventBeginPlay
  (Input|AddMappingContext (PlayerController|LocalPlayerSubsystems|GetEnhancedInputLocalPlayerSubsystem) "/Game/Input/IMC_Default.IMC_Default" 0 "(bIgnoreAllPressedKeysUntilRelease=True,bForceImmediately=False,bNotifyUserSettings=False)")
  (bind _returnvalue (UserInterface|CreateWidget "/Game/UI/WBP_Interface.WBP_Interface_C" self))
  (bind _output_get (Variables|Default|SetInterfaceRef _returnvalue))
  (bind _returnvalue_2 (Actor|GetActorOfClass "/Script/GDF270.VoxelWorld"))
  (Variables|Default|SetVoxelWorldRef _returnvalue_2)
  (bind _asbp_main_character (Utilities|Casting|CastToBP_MainCharacter (Game|Player|GetPlayerPawn 0)))
  (Variables|Default|SetMainCharacterRef _asbp_main_character))

(event EventTick
  (params (DeltaSeconds :type Float%20%28single-precision%29))
  (CallFunction|DisplayDebug))

(fn ConstructionScript)

(fn DisplayDebug
  (bind _voxelworldref (Variables|Default|GetVoxelWorldRef))
  (bind _voxelworldref_2 (Variables|Default|GetVoxelWorldRef))
  (bind _returnvalue (Class|VoxelWorld|GetPlayerCellCoordinate _voxelworldref))
  (bind _returnvalue_2 (Class|VoxelWorld|GetPlayerSectorCoordinate _voxelworldref_2))
  (bind (_x _y _z) (Utilities|Struct|BreakIntVector _returnvalue))
  (bind (_x_2 _y_2) (Utilities|Struct|BreakIntVector2 _returnvalue_2))
  (Variables|/Script/UMG.TextBlock|SetText (Variables|/Game/UI/WBP_Interface.WBP_Interface_C|GetTextLine1 (Variables|Default|GetInterfaceRef)) (Utilities|Text|FormatText "Cell: {0} {1} {2}" _x _y _z))
  (Variables|/Script/UMG.TextBlock|SetText (Variables|/Game/UI/WBP_Interface.WBP_Interface_C|GetTextLine2 (Variables|Default|GetInterfaceRef)) (Utilities|Text|FormatText "Sector: {0} {1}" _x_2 _y_2))
  (switch Utilities|FlowControl|Switch|SwitchonEMovementKind (Variables|/Game/Player/BP_MainCharacter.BP_MainCharacter_C|GetMovementKind (Variables|Default|GetMainCharacterRef))
    (:NewEnumerator0
      (Variables|/Script/UMG.TextBlock|SetText (Variables|/Game/UI/WBP_Interface.WBP_Interface_C|GetTextLine3 (Variables|Default|GetInterfaceRef)) "Movement: Ground"))
    (:NewEnumerator1
      (Variables|/Script/UMG.TextBlock|SetText (Variables|/Game/UI/WBP_Interface.WBP_Interface_C|GetTextLine3 (Variables|Default|GetInterfaceRef)) "Movement: Air"))))