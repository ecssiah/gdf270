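; Player character Blueprint that moves either on the ground or in free flight, starting airborne and toggling via an input action.
; Enhanced Input events delegate to move, look, jump and use functions, with use only printing its value as a placeholder.
; SetMovementKind switches the movement component between Walking and gravity-free Flying.
; Movement input is relative to the actor's axes, adding the vertical component only in Air.
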(event Input|EnhancedActionEvents|EnhancedInputActionIA_Move
  (params (ActionValue :type Vector :default "0, 0, 0") (ElapsedSeconds :type Float%20%28double-precision%29) (TriggeredSeconds :type Float%20%28double-precision%29) (InputAction :type Input%20Action%20Object%20Reference :default "/Game/Input/IA_Move.IA_Move"))
  (CallFunction|MoveAction ActionValue))

(event Input|EnhancedActionEvents|EnhancedInputActionIA_Look
  (params (ActionValue :type Vector%202D%20Structure) (ElapsedSeconds :type Float%20%28double-precision%29) (TriggeredSeconds :type Float%20%28double-precision%29) (InputAction :type Input%20Action%20Object%20Reference :default "/Game/Input/IA_Look.IA_Look"))
  (CallFunction|LookAction ActionValue))

(event Input|EnhancedActionEvents|EnhancedInputActionIA_Jump
  (params (ActionValue :type Boolean) (ElapsedSeconds :type Float%20%28double-precision%29) (TriggeredSeconds :type Float%20%28double-precision%29) (InputAction :type Input%20Action%20Object%20Reference :default "/Game/Input/IA_Jump.IA_Jump"))
  (:Started
    (CallFunction|JumpAction ActionValue :!label _label))
  (:Canceled
    (goto _label))
  (:Completed
    (goto _label)))

(event Input|EnhancedActionEvents|EnhancedInputActionIA_Use
  (params (ActionValue :type Boolean) (ElapsedSeconds :type Float%20%28double-precision%29) (TriggeredSeconds :type Float%20%28double-precision%29) (InputAction :type Input%20Action%20Object%20Reference :default "/Game/Input/IA_Use.IA_Use"))
  (:Started
    (CallFunction|UseAction ActionValue)))

(event Input|EnhancedActionEvents|EnhancedInputActionIA_SwitchMovement
  (params (ActionValue :type Boolean) (ElapsedSeconds :type Float%20%28double-precision%29) (TriggeredSeconds :type Float%20%28double-precision%29) (InputAction :type Input%20Action%20Object%20Reference :default "/Game/Input/IA_SwitchMovement.IA_SwitchMovement"))
  (:Started
    (switch Utilities|FlowControl|Switch|SwitchonEMovementKind (Variables|Default|GetMovementKind)
      (:NewEnumerator0
        (Variables|Default|SetMovementKind "NewEnumerator1")
        (CallFunction|SetMovementKind "NewEnumerator1"))
      (:NewEnumerator1
        (Variables|Default|SetMovementKind "NewEnumerator0")
        (CallFunction|SetMovementKind "NewEnumerator0")))))

(event EventBeginPlay
  (Variables|Default|SetMovementKind "NewEnumerator1")
  (CallFunction|SetMovementKind (Variables|Default|GetMovementKind)))

(fn ConstructionScript)

(fn MoveAction
  (params (InActionValue :type Vector))
  (bind (_x _y) (Math|Vector|BreakVector InActionValue))
  (bind (_x_2 _y_2 _z) (Math|Vector|BreakVector InActionValue))
  (switch Utilities|FlowControl|Switch|SwitchonEMovementKind (Variables|Default|GetMovementKind)
    (:NewEnumerator0
      (Pawn|Input|AddMovementInput (Math|Vector|Normalize (+ (* _x (Transformation|GetActorRightVector)) (* _y (Transformation|GetActorForwardVector)))) 1.0 false))
    (:NewEnumerator1
      (Pawn|Input|AddMovementInput (Math|Vector|Normalize (+ (* _x_2 (Transformation|GetActorRightVector)) (* _y_2 (Transformation|GetActorForwardVector)) (* _z (Transformation|GetActorUpVector)))) 1.0 false))))

(fn LookAction
  (params (ActionValue :type Vector%202D%20Structure))
  (bind (_x _y) (Math|Vector2D|BreakVector2D ActionValue))
  (Pawn|Input|AddControllerYawInput _x)
  (Pawn|Input|AddControllerPitchInput _y))

(fn JumpAction
  (params (ActionValue :type Boolean))
  (if ActionValue
    (Character|Jump)
    (else
      (Character|StopJumping))))

(fn UseAction
  (params (ActionValue :type Boolean))
  (Development|PrintString (Utilities|String|ToString(Text) (Utilities|Text|FormatText "Use: {0}" ActionValue))))

(fn SetMovementKind
  (params (InMovementKind :type EMovementKind%20Enum :default "NewEnumerator0"))
  (switch Utilities|FlowControl|Switch|SwitchonEMovementKind InMovementKind
    (:NewEnumerator0
      (Pawn|Components|CharacterMovement|SetMovementMode (Variables|Character|GetCharacterMovement) "MOVE_Walking" 0)
      (Variables|/Script/Engine.CharacterMovementComponent|SetGravityScale (Variables|Character|GetCharacterMovement) 2.0))
    (:NewEnumerator1
      (Pawn|Components|CharacterMovement|SetMovementMode (Variables|Character|GetCharacterMovement) "MOVE_Flying" 0)
      (Variables|/Script/Engine.CharacterMovementComponent|SetGravityScale (Variables|Character|GetCharacterMovement) 0.0))))